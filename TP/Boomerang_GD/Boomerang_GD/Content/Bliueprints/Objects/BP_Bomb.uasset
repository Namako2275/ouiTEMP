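; BP_Bomb is a bomb object that a boomerang can drag along and that disappears when it touches the player.
; A hitbox overlap with BP_Boomerang stores that actor and sets CanReturn, while an overlap with BP_Player destroys the bomb.
; Once CanReturn is set, Tick moves the bomb toward the boomerang's current location at ReturnSpeed, scaled by delta time.
; No explosion or reward logic is present.
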(event OnComponentBeginOverlap(Hitbox)
  (params (OverlappedComponent :type Primitive%20Component%20Object%20Reference) (OtherActor :type Actor%20Object%20Reference) (OtherComp :type Primitive%20Component%20Object%20Reference) (OtherBodyIndex :type Integer) (bFromSweep :type Boolean) (SweepResult :type Hit%20Result%20Structure%20%28by%20ref%29))
  (Utilities|FlowControl|Sequence
    (:then_0
      (bind _asbp_boomerang (Utilities|Casting|CastToBP_Boomerang OtherActor))
      (Variables|Default|SetCanReturn? true))
    (:then_1
      (Utilities|Casting|CastToBP_Player OtherActor)
      (Actor|DestroyActor))))

(event EventTick
  (params (DeltaSeconds :type Float%20%28single-precision%29))
  (bind _self self)
  (bind _returnvalue (Transformation|GetActorLocation _self))
  (if (Variables|Default|GetCanReturn?)
    (Transformation|SetActorLocation (Math|Vector|MakeVector (.x (+ _returnvalue (* (* (Math|Vector|Normalize (- (Transformation|GetActorLocation (stale OnComponentBeginOverlap(Hitbox) _asbp_boomerang)) _returnvalue)) (Variables|Default|GetReturnSpeed)) DeltaSeconds))) (.y (+ _returnvalue (* (* (Math|Vector|Normalize (- (Transformation|GetActorLocation (stale OnComponentBeginOverlap(Hitbox) _asbp_boomerang)) _returnvalue)) (Variables|Default|GetReturnSpeed)) DeltaSeconds))) (.z (+ _returnvalue (* (* (Math|Vector|Normalize (- (Transformation|GetActorLocation (stale OnComponentBeginOverlap(Hitbox) _asbp_boomerang)) _returnvalue)) (Variables|Default|GetReturnSpeed)) DeltaSeconds)))) false false)))

(fn ConstructionScript)