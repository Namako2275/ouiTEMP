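; Spawner actor that places bombs at its own location.
; A looping timer, started on BeginPlay, spawns a BP_Bomb every two seconds unless a flag says one is already there.
; The Detect component sets that flag only on begin overlap: true for a bomb, false for any other actor, with no end-overlap reset.
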(event OnComponentBeginOverlap(Detect)
  (params (OverlappedComponent :type Primitive%20Component%20Object%20Reference) (OtherActor :type Actor%20Object%20Reference) (OtherComp :type Primitive%20Component%20Object%20Reference) (OtherBodyIndex :type Integer) (bFromSweep :type Boolean) (SweepResult :type Hit%20Result%20Structure%20%28by%20ref%29))
  (Utilities|Casting|CastToBP_Bomb OtherActor
    (:then
      (Variables|Default|SetBombAlreadyThere? true))
    (:CastFailed
      (Variables|Default|SetBombAlreadyThere? false))))

(event Custom|SpawnBomb
  (if (not (Variables|Default|GetBombAlreadyThere?))
    (Game|SpawnActorfromClass "/Game/Blueprints/Objects/BP_Bomb.BP_Bomb_C" (Math|Transform|MakeTransform (Transformation|GetActorLocation self) "0, 0, 0" "1.000000,1.000000,1.000000") "Undefined" "MultiplyWithRoot" 0 0)))

(event EventBeginPlay
  (Utilities|Time|SetTimerbyEvent (delegate Custom|SpawnBomb) 2.0 true))

(fn ConstructionScript)