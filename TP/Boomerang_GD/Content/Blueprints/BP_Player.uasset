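; Player character that moves with Enhanced Input, aims at the mouse cursor and throws boomerangs, with a cursor widget added on BeginPlay.
; Each tick, a cursor hit trace sets the mesh yaw, offset for control rotation, and stores CharacterBaseRotation.
; Shooting spawns a half-scale boomerang with that rotation and clears CanThrow, which this graph never resets.
; An older deprojection-based launch velocity chain is left disconnected.
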(event Custom|SetMeshRotationToCursor
  (bind _returnvalue (Game|GetPlayerController 0))
  (bind _returnvalue_2 (Transformation|GetActorLocation))
  (bind _hitresult (Game|Player|GetHitResultUnderCursorbyChannel _returnvalue "TraceTypeQuery3" true))
  (bind _impactpoint (Collision|BreakHitResult _hitresult))
  (bind _returnvalue_3 (Math|Rotator|FindLookatRotation _returnvalue_2 _impactpoint))
  (bind _yaw (Math|Rotator|BreakRotator _returnvalue_3))
  (bind _output_get (Variables|Default|SetMouse_Location (- (- _yaw 9e+01) (.yaw (Pawn|GetControlRotation :!class /Script/Engine.Pawn)))))
  (Transformation|SetRelativeRotation (Variables|Character|GetMesh) (Math|Rotator|MakeRotator 0.0 0.0 _output_get) false false)
  (Variables|Default|SetCharacterBaseRotation (Math|Rotator|MakeRotator 0.0 0.0 _yaw)))

(event Input|EnhancedActionEvents|EnhancedInputActionIA_Move
  (params (ActionValue :type Vector%202D%20Structure) (ElapsedSeconds :type Float%20%28double-precision%29) (TriggeredSeconds :type Float%20%28double-precision%29) (InputAction :type Input%20Action%20Object%20Reference :default "/Game/Inputs/IA_Move.IA_Move"))
  (Pawn|Input|AddMovementInput (Transformation|GetActorRightVector) (.x ActionValue) false)
  (Pawn|Input|AddMovementInput (Transformation|GetActorForwardVector) (.y ActionValue) false))

(event Input|EnhancedActionEvents|EnhancedInputActionIA_Shoot
  (params (ActionValue :type Boolean) (ElapsedSeconds :type Float%20%28double-precision%29) (TriggeredSeconds :type Float%20%28double-precision%29) (InputAction :type Input%20Action%20Object%20Reference :default "/Game/Inputs/IA_Shoot.IA_Shoot"))
  (bind _self self)
  (bind _returnvalue (Transformation|GetActorLocation _self))
  (:Started
    (if (Variables|Default|GetCanThrow?)
      (Variables|Default|SetCanThrow? false)
      (Game|SpawnActorfromClass (Variables|Default|GetBP_Boomerang) (Math|Transform|MakeTransform (Math|Vector|MakeVector (.x _returnvalue) (.y _returnvalue) (.z _returnvalue)) (Variables|Default|GetCharacterBaseRotation) "0.500000,0.500000,0.500000") "Undefined" "MultiplyWithRoot" 0 0))))

(event EventBeginPlay
  (bind _returnvalue (Game|GetPlayerController 0))
  (Input|AddMappingContext (PlayerController|LocalPlayerSubsystems|GetEnhancedInputLocalPlayerSubsystem _returnvalue) "/Game/Inputs/IMC_Player.IMC_Player" 0 "(bIgnoreAllPressedKeysUntilRelease=True,bForceImmediately=False,bNotifyUserSettings=False)")
  (bind _returnvalue_2 (UserInterface|CreateWidget "/Game/Widgets/WBP_Cursor.WBP_Cursor_C" _returnvalue))
  (UserInterface|Viewport|AddtoViewport _returnvalue_2 0))

(event EventTick
  (params (DeltaSeconds :type Float%20%28single-precision%29))
  (CallFunction|SetMeshRotationtoCursor))

(fn ConstructionScript)