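; Boomerang projectile that flies out from the player, then homes back to them and re-enables throwing on arrival.
; Projectile movement drives the outward flight until the player's max flight time elapses or the hitbox overlaps a component not tagged GoThrough, which also plays an impact sound.
; Tick then moves it toward the player at ReturnSpeed, destroying it when close.
; A looping-style whoosh sound starts once in flight and stops on catch.
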(event OnComponentBeginOverlap(Hitbox)
  (params (OverlappedComponent :type Primitive%20Component%20Object%20Reference) (OtherActor :type Actor%20Object%20Reference) (OtherComp :type Primitive%20Component%20Object%20Reference) (OtherBodyIndex :type Integer) (bFromSweep :type Boolean) (SweepResult :type Hit%20Result%20Structure%20%28by%20ref%29))
  (if (not (Components|ComponentHasTag OtherComp "GoThrough"))
    (Audio|PlaySoundatLocation "/Game/Sounds/ribhavagrawal-hit-by-a-wood-230542.ribhavagrawal-hit-by-a-wood-230542" (Transformation|GetWorldLocation OtherComp) "0, 0, 0" 1.0 1.0 0.22 "/Game/Sounds/SA_Boomerang.SA_Boomerang" 0 0 0)
    (Variables|Default|SetIsFlying? false)
    (Components|Activation|Deactivate (Variables|Default|GetProjectileMovement))))

(event Custom|Parameters
  (bind _asbp_player (Utilities|Casting|CastToBP_Player (Game|GetPlayerCharacter 0)))
  (Variables|Default|SetMaxFlightTime (Variables|/Game/Blueprints/BP_Player.BP_Player_C|GetMaxFlight _asbp_player)))

(event EventBeginPlay
  (CallFunction|Parameters)
  (Variables|Default|SetStartTick true)
  (Components|Activation|Activate (Variables|Default|GetProjectileMovement) false))

(event EventTick
  (params (DeltaSeconds :type Float%20%28single-precision%29))
  (bind _returnvalue (Game|GetPlayerCharacter 0))
  (bind _returnvalue_2 (Game|GetPlayerCharacter 0))
  (bind _self self)
  (bind _returnspeed (Variables|Default|GetReturnSpeed))
  (bind _returnvalue_3 (Transformation|GetActorLocation _self))
  (bind _returnvalue_4 (Transformation|GetActorLocation _returnvalue_2))
  (bind _returnvalue_5 (- _returnvalue_4 _returnvalue_3))
  (bind _returnvalue_6 (Math|Vector|Normalize _returnvalue_5))
  (bind _returnvalue_7 (* _returnvalue_6 _returnspeed))
  (bind _returnvalue_8 (* _returnvalue_7 DeltaSeconds))
  (bind _returnvalue_9 (+ _returnvalue_3 _returnvalue_8))
  (if (Variables|Default|GetStartTick)
    (Variables|Default|SetCurrentFlightTime (+ DeltaSeconds (Variables|Default|GetCurrentFlightTime)))
    (if (Variables|Default|GetIsFlying?)
      (Utilities|FlowControl|Sequence
        (:then_0
          (Utilities|FlowControl|DoOnce false
            (:Completed
              (bind _returnvalue_10 (Audio|CreateSound2D "/Game/Sounds/floraphonic-spin-whoosh-2-186597.floraphonic-spin-whoosh-2-186597" 1.0 1.0 0.0 0))
              (Audio|Components|Audio|Play _returnvalue_10 0.0))))
        (:then_1
          (if (>= (Variables|Default|GetCurrentFlightTime) (Variables|Default|GetMaxFlightTime))
            (Variables|Default|SetIsFlying? false)
            (Components|Activation|Deactivate (Variables|Default|GetProjectileMovement)))))
      (else
        (Transformation|SetActorLocation (Math|Vector|MakeVector (.x _returnvalue_9) (.y _returnvalue_9) (.z _returnvalue_9)) false false)
        (if (< (Math|Vector|Distance(Vector) _returnvalue_3 (Transformation|GetActorLocation _returnvalue)) 1e+01)
          (Audio|Components|Audio|Stop _returnvalue_10)
          (bind _asbp_player (Utilities|Casting|CastToBP_Player _returnvalue))
          (Variables|/Game/Blueprints/BP_Player.BP_Player_C|SetCanThrow? _asbp_player true)
          (Actor|DestroyActor))))))

(fn ConstructionScript)